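; Interactable door Blueprint that slides its Cube mesh vertically to open and close.
; AnimateDoor toggles IsClosed and plays or reverses a Timeline that scales the Cube's relative Z offset.
; CanInteract overrides the parent check, either deferring to it when UseParentImplementation is set or requiring the interacting actor's class to exactly match AcceptableInteractionSource.
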(event EventAnimateDoor
  (if (Variables|Default|GetIsClosed)
    (Variables|Default|SetIsClosed (not (Variables|Default|GetIsClosed)))
    (bind _newtrack_0 (Timeline|Timeline Play)
      (:Update
        _)
      (:Finished
        _))
    (Transformation|SetRelativeLocation (Variables|Default|GetCube) (* _newtrack_0 (Math|Vector|MakeVector 0.0 0.0 2e+02)) false false)
    (else
      (Variables|Default|SetIsClosed (not (Variables|Default|GetIsClosed)))
      (Timeline|Timeline Reverse))))

(fn ConstructionScript)

(fn CanInteract
  (params (InteractingActor :type Actor%20Object%20Reference))
  ;[1 1 1] Example of us being able to use eithe rthe parent implementation or overriding it complety to do what we want to do, in this case I just want to return true at all times if we arent using the parent implementation in cpp, which ensures only characters are allowed to interact with the door
  (if (Variables|Default|GetUseParentImplementation)
    (bind _returnvalue (|CallParentFunction InteractingActor))
    (return _returnvalue)
    (else
      (return (== (Utilities|GetClass InteractingActor) (Variables|Default|GetAcceptableInteractionSource))))))